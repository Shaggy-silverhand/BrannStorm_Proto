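; BP_Item is an item actor that shows one of two interact icons based on the player character's proximity.
; Its construction script sizes two collision spheres with crossed names: OuterSphereCollision takes InnerSphereRadius and InnerSphereCollision takes OuterSphereRadius.
; Entering InnerSphereCollision shows the outer icon and leaving it hides both.
; Entering OuterSphereCollision swaps to the inner icon and leaving it restores the outer one.
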(event OnComponentBeginOverlap(outerSphereCollision)
  (params (OverlappedComponent :type Primitive%20Component%20Object%20Reference) (OtherActor :type Actor%20Object%20Reference) (OtherComp :type Primitive%20Component%20Object%20Reference) (OtherBodyIndex :type Integer) (bFromSweep :type Boolean) (SweepResult :type Hit%20Result%20Structure%20%28by%20ref%29))
  (if (== OtherActor (Game|GetPlayerCharacter 0))
    (Development|SetHiddeninGame (Variables|Default|GetinnerInteractIcon) false false)
    (Development|SetHiddeninGame (Variables|Default|GetouterInteractIcon) true false)))

(event OnComponentEndOverlap(outerSphereCollision)
  (params (OverlappedComponent :type Primitive%20Component%20Object%20Reference) (OtherActor :type Actor%20Object%20Reference) (OtherComp :type Primitive%20Component%20Object%20Reference) (OtherBodyIndex :type Integer))
  (if (== (Game|GetPlayerCharacter 0) OtherActor)
    (Development|SetHiddeninGame (Variables|Default|GetinnerInteractIcon) true false)
    (Development|SetHiddeninGame (Variables|Default|GetouterInteractIcon) false false)))

(event OnComponentBeginOverlap(innerSphereCollision)
  (params (OverlappedComponent :type Primitive%20Component%20Object%20Reference) (OtherActor :type Actor%20Object%20Reference) (OtherComp :type Primitive%20Component%20Object%20Reference) (OtherBodyIndex :type Integer) (bFromSweep :type Boolean) (SweepResult :type Hit%20Result%20Structure%20%28by%20ref%29))
  (if (== OtherActor (Game|GetPlayerCharacter 0))
    (Development|SetHiddeninGame (Variables|Default|GetinnerInteractIcon) true false)
    (Development|SetHiddeninGame (Variables|Default|GetouterInteractIcon) false false)))

(event OnComponentEndOverlap(innerSphereCollision)
  (params (OverlappedComponent :type Primitive%20Component%20Object%20Reference) (OtherActor :type Actor%20Object%20Reference) (OtherComp :type Primitive%20Component%20Object%20Reference) (OtherBodyIndex :type Integer))
  (if (== (Game|GetPlayerCharacter 0) OtherActor)
    (Development|SetHiddeninGame (Variables|Default|GetinnerInteractIcon) true false)
    (Development|SetHiddeninGame (Variables|Default|GetouterInteractIcon) true false)))

(fn ConstructionScript
  (Components|Sphere|SetSphereRadius (Variables|Default|GetouterSphereCollision) (Variables|Public|GetInnerSphereRadius) true)
  (Components|Sphere|SetSphereRadius (Variables|Default|GetinnerSphereCollision) (Variables|Public|GetouterSphereRadius) true))