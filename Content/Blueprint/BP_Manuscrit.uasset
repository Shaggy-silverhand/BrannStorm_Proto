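; BP_Manuscrit is an interactable manuscript that the player picks up to view on screen and lays back down.
; Its Interaction event alternates through a FlipFlop between the two states.
; Picking up creates a new WG_Manuscrit widget, hides the mesh and blocks player look and move input.
; Laying down calls LayDownManuscrit on that widget, shows the mesh again and restores input.
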(event EventInteraction
  (params (Component :type Primitive%20Component%20Object%20Reference) (RotateLeft :type Boolean))
  (bind _returnvalue (Game|GetPlayerController 0))
  (bind _staticmeshcomponent0 (Variables|Default|GetStaticMeshComponent0))
  (Utilities|FlowControl|FlipFlop
    (:A
      (bind _returnvalue_2 (UserInterface|CreateWidget "/Game/Blueprint/WG_Manuscrit.WG_Manuscrit_C"))
      (UserInterface|Viewport|AddtoViewport _returnvalue_2 0)
      (Input|SetIgnoreLookInput _returnvalue true)
      (Input|SetIgnoreMoveInput _returnvalue true)
      (Rendering|SetVisibility _staticmeshcomponent0 false false))
    (:B
      (Default|LayDownManuscrit _returnvalue_2)
      (Input|SetIgnoreLookInput _returnvalue false)
      (Input|SetIgnoreMoveInput _returnvalue false)
      (Rendering|SetVisibility _staticmeshcomponent0 true false))))

(fn ConstructionScript)