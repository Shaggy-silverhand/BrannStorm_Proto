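; Armory door Blueprint that opens on interaction only when the player's third-person character has the key.
; With the key, it reveals and rotates the key mesh while a timeline swings the door open, alongside a world camera shake call.
; Without it, a short timeline jiggles the door slightly, gated by a DoOnce that resets when the shake finishes.
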(event EventInteraction
  (params (Component :type Primitive%20Component%20Object%20Reference) (RotateLeft :type Boolean))
  (bind _asbp_third_person_character (Utilities|Casting|CastToBP_ThirdPersonCharacter (Game|GetPlayerCharacter 0)))
  (if (Variables|/Game/ThirdPerson/Blueprints/BP_ThirdPersonCharacter.BP_ThirdPersonCharacter_C|Getkey _asbp_third_person_character)
    (Utilities|FlowControl|Sequence
      (:then_0
        (Development|SetHiddeninGame (Variables|Default|Getkeys) false false)
        (bind _opening (Timeline|key%20timeline Play)
          (:Update
            (Transformation|SetRelativeRotation (Variables|Default|Getkeys) (Math|Rotator|MakeRotator 0.0 (Math|Float|Lerp -85.0 -0.0 _opening) -85.0) false false))))
      (:then_1
        (Camera|PlayWorldCameraShake 0 (Transformation|GetWorldLocation (Variables|Default|GetScene)) 0.0 5e+02)
        (bind _door (Timeline|Timeline_0 Play)
          (:Update
            (Transformation|SetRelativeRotation (Variables|Default|Getdoor) (Math|Rotator|MakeRotator 0.0 0.0 (Math|Float|Lerp 0.0 45.0 _door)) false false)))))
    (else
      (Utilities|FlowControl|DoOnce false :!label _label
        (:Completed
          (bind _shake (Timeline|Timeline PlayFromStart)
            (:Update
              (Transformation|SetRelativeRotation (Variables|Default|Getdoor) (Math|Rotator|MakeRotator 0.0 0.0 (Math|Float|Lerp 0.0 2.0 _shake)) false false))
            (:Finished
              (goto _label Reset))))))))

(fn ConstructionScript)