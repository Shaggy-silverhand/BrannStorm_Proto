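; BP_Socle is an interactable pedestal that takes the player's idol and opens a linked door.
; On interaction, it checks the player character's Idol state; without it, the DoOnce resets so the pedestal can be used again.
; With it, the idol mesh is revealed and a timeline lowers it along Z from its stored start position in X and Y.
; When the timeline finishes, it calls OpenDoor on the referenced door.
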(event EventInteraction
  (params (Component :type Primitive%20Component%20Object%20Reference) (RotateLeft :type Boolean))
  (bind _relative_location (Variables|Default|GetRelative%20Location))
  (Utilities|FlowControl|DoOnce false :!label _label
    (:Completed
      (bind _asbp_third_person_character (Utilities|Casting|CastToBP_ThirdPersonCharacter (Game|GetPlayerCharacter 0)))
      (if (Variables|/Game/ThirdPerson/Blueprints/BP_ThirdPersonCharacter.BP_ThirdPersonCharacter_C|GetIdol _asbp_third_person_character)
        (Development|SetHiddeninGame (Variables|Default|Getidol) false false)
        (bind _idolspawning (Timeline|Timeline Play)
          (:Update
            (Transformation|SetRelativeLocation (Variables|Default|Getidol) (Math|Vector|MakeVector (.x _relative_location) (.y _relative_location) (Math|Float|Lerp 45.0 5.0 _idolspawning)) false false))
          (:Finished
            (Default|OpenDoor (Variables|Default|GetDoorRef))))
        (else
          (goto _label Reset))))))

(event EventBeginPlay
  (Variables|Default|SetRelative%20Location (Variables|/Script/Engine.SceneComponent|GetRelativeLocation (Variables|Default|Getidol))))

(fn ConstructionScript)