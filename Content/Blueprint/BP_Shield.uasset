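; BP_Shield is a rotation-code puzzle that opens a linked Chest when the Green, Red, Blue and Yellow components are turned to the correct angles.
; Rotate yaws a given component by RotateValue only when RotateLeft is true, then calls CheckCode.
; CheckCode compares that component's relative yaw with its Code entry within a tolerance, stores the result in CodeIsGood, and calls OpenChest once every entry is true.
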(event EventBeginPlay)

(event Collision|EventActorBeginOverlap
  (params (OtherActor :type Actor%20Object%20Reference)))

(event EventTick
  (params (DeltaSeconds :type Float%20%28single-precision%29)))

(fn ConstructionScript)

(fn Rotate
  (params (Component :type Primitive%20Component%20Object%20Reference) (RotateLeft :type Boolean))
  (if RotateLeft
    (Transformation|AddRelativeRotation Component (Math|Rotator|MakeRotator 0.0 0.0 (Variables|Default|GetRotateValue)) false false)
    (CallFunction|CheckCode Component)))

(fn CheckCode
  (params (Component :type Primitive%20Component%20Object%20Reference))
  (if (== Component (Variables|Default|GetGreen))
    (LocalVariables|SetSelectedMesh 0)
    (Utilities|Array|SetArrayElem (Variables|Default|GetCodeIsGood) (LocalVariables|GetSelectedMesh) (Math|Float|NearlyEqual(Float) (Utilities|Array|Get(acopy) (Variables|Default|GetCode) (LocalVariables|GetSelectedMesh)) (.yaw (Variables|/Script/Engine.SceneComponent|GetRelativeRotation Component)) 1.0) :!label _label)
    (bind _array_element (Utilities|Array|ForEachLoopwithBreak (Variables|Default|GetCodeIsGood) :!label _label_2)
      (:LoopBody
        (if (not _array_element)
          (LocalVariables|SetLocalFailed true)
          (goto _label_2 Break)))
      (:Completed
        (if (not (LocalVariables|GetLocalFailed))
          (Default|OpenChest (Variables|Default|GetChest)))))
    (elif (== Component (Variables|Default|GetRed))
      (LocalVariables|SetSelectedMesh 1)
      (goto _label)
      (elif (== Component (Variables|Default|GetBlue))
        (LocalVariables|SetSelectedMesh 2)
        (goto _label)
        (elif (== Component (Variables|Default|GetYellow))
          (LocalVariables|SetSelectedMesh 3)
          (goto _label))))))