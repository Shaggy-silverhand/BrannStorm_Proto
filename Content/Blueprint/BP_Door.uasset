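; BP_Door is a door that can swing open or rattle in place when interacted with.
; The Opendoor event plays a world camera shake at the door and runs a timeline that rotates the mesh's yaw partway open.
; The Interaction event plays a separate shake timeline for a slight yaw wobble, using a DoOnce that resets on finish so the rattle cannot restart mid-play.
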(event Custom|Open%20door
  (Camera|PlayWorldCameraShake 0 (Transformation|GetWorldLocation (Variables|Default|GetScene)) 0.0 5e+02)
  (bind _door (Timeline|Timeline Play)
    (:Update
      (Transformation|SetRelativeRotation (Variables|Default|GetStaticMeshComponent0) (Math|Rotator|MakeRotator 0.0 0.0 (Math|Float|Lerp 0.0 45.0 _door)) false false))))

(event EventInteraction
  (params (Component :type Primitive%20Component%20Object%20Reference) (RotateLeft :type Boolean))
  (Utilities|FlowControl|DoOnce false :!label _label
    (:Completed
      (bind _shake (Timeline|Door_Shake PlayFromStart)
        (:Update
          (Transformation|SetRelativeRotation (Variables|Default|GetStaticMeshComponent0) (Math|Rotator|MakeRotator 0.0 0.0 (Math|Float|Lerp 0.0 2.0 _shake)) false false))
        (:Finished
          (goto _label Reset))))))

(fn ConstructionScript)